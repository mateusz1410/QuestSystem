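; BP_LocationMarker is a quest location trigger that reports when the player character reaches it.
; On sphere overlap by a ThirdPersonCharacter, it calls LocationReached on every quest in that character's QuestLog, passing itself.
; The sphere's collision is disabled inside that loop, so the marker stops triggering once any quest is notified.
; An unconnected leftover loop compares incomplete objectives against a location name.
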(event `self.Sphere.OnComponentBeginOverlap`
  (params (OverlappedComponent :type "PrimitiveComponent Object Reference") (OtherActor :type "Actor Object Reference") (OtherComp :type "PrimitiveComponent Object Reference") (OtherBodyIndex :type Integer) (bFromSweep :type Boolean) (SweepResult :type "HitResult Structure (by ref)"))
  (bind _asthird_person_character (cast `/Game/ThirdPersonBP/Blueprints/ThirdPersonCharacter` OtherActor))
  (for _array_element (`/Game/BP/QuestSystem/BP_QuestLog.Quests` (`/Game/ThirdPersonBP/Blueprints/ThirdPersonCharacter.QuestLog` _asthird_person_character))
    (`/Game/BP/QuestSystem/Quests/BP_Quest.LocationReached` _array_element self)
    (`PrimitiveComponent.SetCollisionEnabled` (`self.Sphere`) "NoCollision")))

(fn `UserConstructionScript`)