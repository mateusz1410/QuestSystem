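; Quest log Blueprint that stores the player's quests and shows or hides the quest log screen.
; AddQuestToLog appends quests without duplicates.
; ToggleQuestLog creates a WDG_QuestLog widget anchored full-stretch on the HUD canvas held by ThirdPersonGameMode, or removes the existing one.
; Toggling also switches between UI-only input with a visible cursor and game-only input with it hidden.
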(fn `AddQuestToLog`
  (params (quest :type "/Game/BP/QuestSystem/Quests/BP_Quest Object Reference"))
  (`KismetArrayLibrary.Array_AddUnique` (`self.Quests`) quest))

(fn `ToggleQuestLog`
  (bind _returnvalue (`GameplayStatics.GetPlayerController` 0))
  (bind _returnvalue_2 (`GameplayStatics.GetPlayerController` 0))
  (bind _wdg_questlog (`self.WDG_QuestLog`) ; ConvertToValidatedGet
    (:`then`
      (`Widget.RemoveFromParent` _wdg_questlog)
      (set `self.WDG_QuestLog` null)
      (`WidgetBlueprintLibrary.SetInputMode_GameOnly` _returnvalue)
      (set `PlayerController.bShowMouseCursor` false _returnvalue))
    (:`else`
      (bind _returnvalue_3 (`|CreateWidget` "/Game/BP/QuestSystem/QuestUI/WDG_questLog.WDG_QuestLog_C"))
      (set `self.WDG_QuestLog` _returnvalue_3)
      (bind _asthird_person_game_mode (cast `/Game/ThirdPersonBP/Blueprints/ThirdPersonGameMode` (`GameplayStatics.GetGameMode`)))
      (bind _returnvalue_4 (`CanvasPanel.AddChildToCanvas` (`/Game/ThirdPersonBP/Blueprints/ThirdPersonGameMode.HUD Canvas` _asthird_person_game_mode) (`self.WDG_QuestLog`)))
      (`CanvasPanelSlot.SetAnchors` _returnvalue_4 (make `Anchors` (0.0 0.0) (1.0 1.0)))
      (`WidgetBlueprintLibrary.SetInputMode_UIOnlyEx` _returnvalue_2 (`self.WDG_QuestLog`) "LockOnCapture")
      (set `PlayerController.bShowMouseCursor` true _returnvalue_2))))