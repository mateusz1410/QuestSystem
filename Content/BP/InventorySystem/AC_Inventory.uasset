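; Inventory component that stores a capacity-limited list of items and opens or closes the inventory screen.
; AddItem stacks by name, adding one to a matching entry's amount or appending a new entry, but only while the list is below Capacity.
; ToggleInventory creates the WDG_Inventory widget with the capacity or removes it, switching input mode and mouse cursor between UI and game.
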(fn `AddItem`
  (params (NewItem :type "/Game/BP/InventorySystem/ItemStruct Structure (by ref)"))
  (locals (IsInArray :type Boolean))
  (bind _items (`self.Items`))
  (bind _returnvalue (`KismetArrayLibrary.Array_Length` _items))
  (if (< _returnvalue (`self.Capacity`))
    (if (> _returnvalue 0)
      (for (_array_element _array_index) _items
        (if (`KismetTextLibrary.EqualEqual_TextText` (break `/Game/BP/InventorySystem/ItemStruct` _array_element) (`.Name_5_9B1562CC46116E79FCFD01A0857A78AA` (break `/Game/BP/InventorySystem/ItemStruct` NewItem)))
          (bind _result (`/Engine/EditorBlueprintResources/StandardMacros.IncrementInt` (`.Amount_19_206DC549445031A0E8DF1593C23DC157` (break `/Game/BP/InventorySystem/ItemStruct` _array_element)))
            (:`  `
              (`KismetArrayLibrary.Array_Set` _items _array_index (make `/Game/BP/InventorySystem/ItemStruct` (break `/Game/BP/InventorySystem/ItemStruct` _array_element) (`.Icon_2_71E18FB8458BC31598FEA7B89BFD011A` (break `/Game/BP/InventorySystem/ItemStruct` _array_element)) (`.Description_12_B7AFA554499331C0788D3985FEF85300` (break `/Game/BP/InventorySystem/ItemStruct` _array_element)) (`.Value_8_23EC8C31405FC1041F3F4C96A87FE408` (break `/Game/BP/InventorySystem/ItemStruct` _array_element)) (`.Actor_16_51718C464E9007FB26F57FA16591B403` (break `/Game/BP/InventorySystem/ItemStruct` _array_element)) _result))
              (set `local.IsInArray` true)
              (break)))))
      (if (not (`local.IsInArray`))
        (`KismetArrayLibrary.Array_Add` (`self.Items`) NewItem :!label _label))
      (else
        (goto _label)))))

(fn `ToggleInventory`
  (bind _returnvalue (`GameplayStatics.GetPlayerController` 0))
  (bind _returnvalue_2 (`GameplayStatics.GetPlayerController` 0))
  (bind _wdg_inventory (`self.WDG_Inventory`)
    (:`then`
      (`Widget.RemoveFromParent` _wdg_inventory)
      (set `self.WDG_Inventory` null)
      (`WidgetBlueprintLibrary.SetInputMode_GameOnly` _returnvalue)
      (set `PlayerController.bShowMouseCursor` false _returnvalue))
    (:`else`
      (bind _returnvalue_3 (`|CreateWidget` "/Game/BP/InventorySystem/InventoryUI/WDG_Inventory.WDG_Inventory_C" null (`self.Capacity`)))
      (bind _output_get (set `self.WDG_Inventory` _returnvalue_3))
      (`UserWidget.AddToViewport` _output_get 0)
      (`WidgetBlueprintLibrary.SetInputMode_UIOnlyEx` _returnvalue_2 _output_get "LockOnCapture")
      (set `PlayerController.bShowMouseCursor` true _returnvalue_2))))