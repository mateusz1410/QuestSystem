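; BP_Item is a pickup actor that adds itself to the player's inventory when interacted with.
; Interact casts player 0's character to ThirdPersonCharacter, passes the GetItem result to its ACInventory AddItem, then sets a very short lifespan to remove the actor.
; GetItem builds a hardcoded test item struct with display data, value, amount and a reference to this actor.
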(event `/Game/BP/QuestSystem/BPI_Interactable.Interact`
  (bind _asthird_person_character (cast `/Game/ThirdPersonBP/Blueprints/ThirdPersonCharacter` (`GameplayStatics.GetPlayerCharacter` 0)))
  (bind _item (`self.GetItem`))
  (`/Game/BP/InventorySystem/AC_Inventory.AddItem` (`/Game/ThirdPersonBP/Blueprints/ThirdPersonCharacter.AC_Inventory` _asthird_person_character) _item)
  (`self.SetLifeSpan` 0.1))

(fn `GetItem`
  (returns (Item :type "/Game/BP/InventorySystem/ItemStruct Structure"))
  (return (make `/Game/BP/InventorySystem/ItemStruct` "Item" "/Engine/EngineResources/AICON-Green.AICON-Green" "Test Item" 10.0 self 1)))

(fn `UserConstructionScript`)